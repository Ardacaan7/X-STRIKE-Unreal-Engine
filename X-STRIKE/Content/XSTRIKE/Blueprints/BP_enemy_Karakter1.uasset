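; BP_enemy_Karakter1 is a side-scroller enemy with flipbook animation that chases and attacks the player character.
; Box overlap sets IsSeePlayer, and Tick then moves it along X, turns the sprite, or stops to animate an attack within range.
; Capsule hits deal damage to whatever is struck, throttled by a one-second DoOnce.
; AnyDamage sets health to damage minus health (reversed subtraction), destroying it at zero or below; health-widget linking never runs.
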(event OnComponentBeginOverlap(Box)
  (params (OverlappedComponent :type Primitive%20Component%20Object%20Reference) (OtherActor :type Actor%20Object%20Reference) (OtherComp :type Primitive%20Component%20Object%20Reference) (OtherBodyIndex :type Integer) (bFromSweep :type Boolean) (SweepResult :type Hit%20Result%20Structure%20%28by%20ref%29))
  (Utilities|Casting|CastToBP_XSTRIKE_Karakter OtherActor)
  (Variables|Default|SetIsSeePlayer true))

(event OnComponentEndOverlap(Box)
  (params (OverlappedComponent :type Primitive%20Component%20Object%20Reference) (OtherActor :type Actor%20Object%20Reference) (OtherComp :type Primitive%20Component%20Object%20Reference) (OtherBodyIndex :type Integer))
  (Variables|Default|SetIsSeePlayer false))

(event OnComponentHit(CapsuleComponent)
  (params (HitComponent :type Primitive%20Component%20Object%20Reference) (OtherActor :type Actor%20Object%20Reference) (OtherComp :type Primitive%20Component%20Object%20Reference) (NormalImpulse :type Vector :default "0, 0, 0") (Hit :type Hit%20Result%20Structure%20%28by%20ref%29))
  (Utilities|FlowControl|DoOnce false :!label _label
    (:Completed
      (Game|Damage|ApplyDamage OtherActor 5.0 0 0)
      (Utilities|FlowControl|Delay 1.0)
      (goto _label Reset))))

(event Custom|FollowPlayer
  (if (< (Transformation|GetDistanceTo (Variables|Default|Getplayerref)) (Variables|Default|GetSaldiriMenzili))
    (Components|Movement|StopMovementImmediately (Variables|Character|GetCharacterMovement))
    (Sprite|SetFlipbook (Variables|Default|GetSprite) "/Game/PaperAssets/enemy/enemy2/attack/Fb_enemy_attack.Fb_enemy_attack")
    (else
      (Math|Float|CompareFloat (.x (Transformation|GetWorldLocation (Variables|/Script/Paper2D.PaperCharacter|GetSprite (Variables|Default|Getplayerref)))) (.x (Transformation|GetWorldLocation (Variables|Default|GetSprite)))
        (:>
          (Pawn|Input|AddMovementInput "1.000000,0.000000,0.000000" 1.0 false)
          (Sprite|SetFlipbook (Variables|Default|GetSprite) "/Game/PaperAssets/enemy/enemy2/run/Fb_enemy2_run.Fb_enemy2_run"))
        (:<
          (Pawn|Input|AddMovementInput "-1.000000,0.000000,0.000000" 1.0 false)
          (Sprite|SetFlipbook (Variables|Default|GetSprite) "/Game/PaperAssets/enemy/enemy2/run/Fb_enemy2_run.Fb_enemy2_run"))))))

(event Custom|ControlRotation
  (bind _sprite (Variables|Default|GetSprite))
  (Math|Float|CompareFloat (.x (Variables|/Script/Engine.MovementComponent|GetVelocity (Variables|Character|GetCharacterMovement))) 0.0
    (:>
      (Transformation|SetRelativeRotation _sprite "0, 0, 0" false false))
    (:<
      (Transformation|SetRelativeRotation _sprite "0.000000,180.000000,0.000000" false false))))

(event EventBeginPlay
  (bind _asbp_xstrike_karakter (Utilities|Casting|CastToBP_XSTRIKE_Karakter (Game|GetPlayerCharacter 0)))
  (Variables|Default|Setplayerref _asbp_xstrike_karakter))

(event EventTick
  (params (DeltaSeconds :type Float%20%28single-precision%29))
  (if (Variables|Default|GetIsSeePlayer)
    (CallFunction|ControlRotation)
    (CallFunction|FollowPlayer)
    (else
      (Components|Movement|StopMovementImmediately (Variables|Character|GetCharacterMovement))
      (Sprite|SetFlipbook (Variables|Default|GetSprite) "/Game/PaperAssets/enemy/enemy2/idle/Fb_enemy2_idle.Fb_enemy2_idle"))))

(event Game|Damage|EventAnyDamage
  (params (Damage :type Float%20%28single-precision%29) (DamageType :type Damage%20Type%20Object%20Reference) (InstigatedBy :type Controller%20Object%20Reference) (DamageCauser :type Actor%20Object%20Reference))
  (bind _output_get (Variables|Default|SetDusmanCan (- Damage (Variables|Default|GetDusmanCan))))
  (if (<= _output_get 0.0)
    (Sprite|SetFlipbook (Variables|Default|GetSprite) "/Game/PaperAssets/enemy/enemy2/death/Fb_enemy2_death.Fb_enemy2_death")
    (Utilities|FlowControl|Delay 1.0)
    (Actor|DestroyActor)))

(fn ConstructionScript)

(fn InitInput
  (bind _asplayer_controller (Utilities|Casting|CastToPlayerController (Pawn|GetController)))
  (Input|AddMappingContext (PlayerController|LocalPlayerSubsystems|GetEnhancedInputLocalPlayerSubsystem _asplayer_controller) "/Game/XSTRIKE/Input/IMC_SideScroller.IMC_SideScroller" 0 "(bIgnoreAllPressedKeysUntilRelease=True,bForceImmediately=False,bNotifyUserSettings=False)"))